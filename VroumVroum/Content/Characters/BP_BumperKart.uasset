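; BP_BumperKart is the bumper kart character Blueprint, driving its drift and weather feedback.
; On BeginPlay it binds to rain and drift update delegates.
; Drift updates toggle the Boost and Smoke components from the BoostDrifting and Drifting flags.
; Rain updates play or stop the Rain component according to the circuit's weather config.
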(event `self.ReceiveBeginPlay`
  (add `self.OnUpdateRain` (delegate `OnUpdateRain_Event_0`))
  (add `self.OnUpdateDrift` (delegate `OnUpdateDrift_Event_0`)))

(event `OnUpdateDrift_Event_0`
  (`ActorComponent.SetActive` (`self.Boost`) (`self.bBoostDrifting`) false)
  (`ActorComponent.SetActive` (`self.Smoke`) (`self.bDrifting`) false))

(event `OnUpdateRain_Event_0`
  (bind _rain (`self.Rain`))
  (if (`WeatherConfig.bRaining` (`Circuit.GetWeatherConfig` (`self.GetCircuit`)))
    (`AudioComponent.Play` _rain 0.0)
    (else
      (`AudioComponent.Stop` _rain))))

(fn `UserConstructionScript`)