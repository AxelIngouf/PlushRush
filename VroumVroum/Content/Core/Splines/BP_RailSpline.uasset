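; BP_RailSpline is a spline actor that builds a rail from spline mesh segments laid along its spline.
; The construction script adds one spline mesh component per pair of neighboring points, attached to TopScene and shaped by their local positions and tangents.
; Each point's roll is converted from degrees to radians to bank the segment ends, with the mesh update deferred until the final setter.
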(fn `UserConstructionScript`
  (bind _spline (`self.Spline`))
  (for _index (range (+ (- (`SplineComponent.GetNumberOfSplinePoints` (`self.Spline`)) 2) 1))
    (bind _returnvalue (`AddComponent|NODE_AddSplineMeshComponent-0` :`bManualAttachment` true))
    (`SceneComponent.K2_AttachToComponent` _returnvalue (`self.TopScene`) "None" "KeepRelative" "KeepRelative" "KeepRelative" true)
    (bind (_location _tangent) (`SplineComponent.GetLocationAndTangentAtSplinePoint` _spline _index "Local"))
    (bind (_location_2 _tangent_2) (`SplineComponent.GetLocationAndTangentAtSplinePoint` _spline (+ _index 1) "Local"))
    (`SplineMeshComponent.SetStartAndEnd` _returnvalue _location _tangent _location_2 _tangent_2 false)
    (`SplineMeshComponent.SetStartRoll` _returnvalue (`KismetMathLibrary.MultiplyByPi` (/ (`SplineComponent.GetRollAtSplinePoint` (`self.Spline`) _index "Local") 180.0)) false)
    (`SplineMeshComponent.SetEndRoll` _returnvalue (`KismetMathLibrary.MultiplyByPi` (/ (`SplineComponent.GetRollAtSplinePoint` (`self.Spline`) (+ _index 1) "Local") 180.0)) true)))